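; Calibrated lighting actor that applies one of several preset HDRI sky environments, chosen by enum, at construction time.
; The enum maps to an index into a settings array, which drives dynamic materials on separate sky and sun domes, the SkyLight cubemap and manual-exposure post process.
; The directional light takes the preset's sun intensity and direction, yawed opposite the sky rotation, which includes a global rotation offset.
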(event `self.ReceiveBeginPlay`)

(fn `GetStructVars`
  (params (`Sky Idx` :type Integer))
  (bind (_hdri_sunremoved _hdri_sunonly _skyscale _sunscale _sundirection _colortemp _exposurecompensation _focaldistance _skyrotation) (break `/Game/Blueprints/Lighting/Calibrated_Sky_Settings` (`|GetArrayItem` (`self.Calibrated Sky Settings`) `Sky Idx`)))
  (set `self.HDRI SUNREMOVED` _hdri_sunremoved)
  (set `self.HDRI SUNONLY` _hdri_sunonly)
  (set `self.Sky Scale` _skyscale)
  (set `self.Sun Scale` _sunscale)
  (set `self.Sun Direction` _sundirection)
  (set `self.Color Temp` _colortemp)
  (set `self.Exposure Compensation` _exposurecompensation)
  (set `self.Focal Distance` _focaldistance)
  (set `self.Sky Rotation` (+ _skyrotation (`self.Sky Rotation (All)`))))

(fn `set dome`
  (params (`Sky Dome` :type "StaticMeshComponent Object Reference") (`Sky Scale` :type "Float (double-precision)") (`Sky Rotation` :type "Float (double-precision)") (HDRI :type "TextureCube Object Reference"))
  ;[1 1 1] Assign Dynamic Material to SkyDome
  (bind _returnvalue (`PrimitiveComponent.CreateDynamicMaterialInstance` `Sky Dome` 0 (`PrimitiveComponent.GetMaterial` `Sky Dome` 0) "None"))
  ;[1 1 1] Set HDRI Intensity
  (`MaterialInstanceDynamic.SetScalarParameterValue` _returnvalue "Intensity" `Sky Scale`)
  ;[1 1 1] Set Rotation of HDRI
  (`MaterialInstanceDynamic.SetScalarParameterValue` _returnvalue "CubemapRotation" `Sky Rotation`)
  ;[1 1 1] Assign HDRI to Skybox
  (`MaterialInstanceDynamic.SetTextureParameterValue` _returnvalue "Skybox" HDRI))

(fn `SetCalibratedLighting`
  (params (sky_idx :type Integer))
  (`self.GetStructVars` sky_idx)
  (`self.set dome` (`self.Sky Dome`) (`self.Sky Scale`) (`self.Sky Rotation`) (`self.HDRI SUNREMOVED`))
  (if (`KismetSystemLibrary.IsValid` (`self.HDRI SUNONLY`))
    (`self.set dome` (`self.Sun Dome`) (`self.Sky Scale`) (`self.Sky Rotation`) (`self.HDRI SUNONLY`))
    (else
      (`self.set dome` (`self.Sun Dome`) (`self.Sky Scale`) (`self.Sky Rotation`))))
  ;[1 1 1] Assign HDRI to SkyLight
  (`SkyLightComponent.SetCubemap` (`self.SkyLight`) (`self.HDRI SUNREMOVED`))
  ;[1 1 1] Assign Post Process Values
  (set `PostProcessComponent.Settings` (make `PostProcessSettings` :`AutoExposureMethod` "AEM_Manual" :`DepthOfFieldMethod` "DOFM_CircleDOF" :`WhiteTemp` (`self.Color Temp`) :`BloomIntensity` 0.1 :`AutoExposureBias` (`self.Exposure Compensation`) :`AmbientOcclusionIntensity` 1.0 :`DepthOfFieldFocalDistance` (`self.Focal Distance`) :`ScreenSpaceReflectionMaxRoughness` 1.0) (`self.PostProcess`))
  ;[1 1 1] Set Directional Light Intensity
  (`LightComponent.SetIntensity` (`self.DirectionalLight`) (`self.Sun Scale`))
  ;[1 1 1] Set Sun Direction
  (`SceneComponent.K2_SetWorldRotation` (`self.DirectionalLight`) (`self.Sun Direction`) false false)
  ;[1 1 1] Allow Rotation of Sun Direction Along Z Axis
  (`SceneComponent.K2_SetWorldRotation` (`self.DirectionalLight`) (`KismetMathLibrary.ComposeRotators` (`self.Sun Direction`) (`KismetMathLibrary.MakeRotator` 0.0 0.0 (* (`self.Sky Rotation`) -1.0))) false false))

(fn `UserConstructionScript`
  (`self.SetCalibratedLighting` (`BlueprintMapLibrary.Map_Find` (`self.Sky Index Map`) (`|GetEnumeratorNameAsString` (`self.Light Enum`)))))